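; Board manager for a board game that moves players between BP_Frame tiles and triggers each landing tile's event.
; On BeginPlay it gathers every frame in the level into a map keyed by frame ID.
; Movement looks up the next or previous frame and delegates the move to the player; at zero moves left, the current frame's event type is dispatched.
; Only forward and backward move events are implemented; the other effects are empty stubs.
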(event `self.ReceiveBeginPlay`
  (`self.GetAllFrames`))

(fn `AddToPlayerMovement`
  (params (player :type "/Game/Blueprint/BP_Player Object Reference") (numberOfMove :type Integer))
  (locals (actualPosition :type Integer) (positionToMove :type Integer))
  (if (> numberOfMove 0)
    (bind _output_get (set `local.actualPosition` (`/Game/Blueprint/BP_Player.playerPosition` (`local.player`))))
    (bind _nextid (`/Game/Blueprint/BP_Frame.ReturnNextID` (`BlueprintMapLibrary.Map_Find` (`self.frameInThisLevel`) _output_get)))
    (set `local.positionToMove` _nextid)
    (`self.MovePlayers` (`local.player`) (`local.positionToMove`) (`local.numberOfMove`))
    (else
      (bind _output_get_2 (set `local.actualPosition` (`/Game/Blueprint/BP_Player.playerPosition` (`local.player`))))
      (`self.OnPlayerOnFrame` (`/Game/Blueprint/BP_Frame.eventType` (`BlueprintMapLibrary.Map_Find` (`self.frameInThisLevel`) _output_get_2)) (`local.player`)))))

(fn `AleaEvent`
  (params (player :type "/Game/Blueprint/BP_Player Object Reference")))

(fn `BackMovePlayers`
  (params (player :type "/Game/Blueprint/BP_Player Object Reference") (IDFrame :type Integer) (numberOfMove :type Integer))
  (locals (position :type "Vector Structure"))
  (bind _output_get (set `local.position` (`self.K2_GetActorLocation` (`BlueprintMapLibrary.Map_Find` (`self.frameInThisLevel`) IDFrame))))
  (`/Game/Blueprint/BP_Player.BackMovePlayer` (`local.player`) _output_get (`local.IDFrame`) (`local.numberOfMove`)))

(fn `DefineBoard`
  (for _array_element (`self.frames`)
    (bind _frameid (`/Game/Blueprint/BP_Frame.ReturnFrameID` _array_element))
    (`BlueprintMapLibrary.Map_Add` (`self.frameInThisLevel`) _frameid _array_element)))

(fn `DoEvent`
  (params (frameType :type "/Game/Datas/Struct_FrameType Structure") (player :type "/Game/Blueprint/BP_Player Object Reference"))
  (bind (_type _value) (break `/Game/Datas/Struct_FrameType` frameType))
  (switch `/Game/Datas/Enum_FrameEvent` _type
    (:`NewEnumerator0`
      (`self.NoEffect` (`local.player`)))
    (:`NewEnumerator1`
      (`self.LoseMoney` _value (`local.player`)))
    (:`NewEnumerator2`
      (`self.EarnMoney` _value (`local.player`)))
    (:`NewEnumerator3`
      (`self.MoveForward` (`local.player`) _value))
    (:`NewEnumerator4`
      (`self.MoveBackward` (`local.player`) _value))
    (:`NewEnumerator5`
      (`self.Teleport` _value (`local.player`)))
    (:`NewEnumerator6`
      (`self.Shop` (`local.player`)))
    (:`NewEnumerator7`
      (`self.AleaEvent` (`local.player`)))
    (:`NewEnumerator8`
      (`self.MiniGameFrame` (`local.player`)))))

(fn `EarnMoney`
  (params (montant :type Integer) (player :type "/Game/Blueprint/BP_Player Object Reference")))

(fn `GetAllFrames`
  ; Une seule fois au départ, c'est un coût acceptable
  (bind _outactors (`GameplayStatics.GetAllActorsOfClass` "/Game/Blueprint/BP_Frame.BP_Frame_C"))
  (set `self.frames` _outactors)
  (`self.DefineBoard`))

(fn `LoseMoney`
  (params (montant :type Integer) (player :type "/Game/Blueprint/BP_Player Object Reference")))

(fn `MiniGameFrame`
  (params (player :type "/Game/Blueprint/BP_Player Object Reference")))

(fn `MoveBackward`
  (params (player :type "/Game/Blueprint/BP_Player Object Reference") (numberOfMove :type Integer))
  (`self.RemoveToPlayerMovement` player numberOfMove))

(fn `MoveForward`
  (params (player :type "/Game/Blueprint/BP_Player Object Reference") (numberOfMove :type Integer))
  (`self.AddToPlayerMovement` player numberOfMove))

(fn `MovePlayers`
  (params (player :type "/Game/Blueprint/BP_Player Object Reference") (IDFrame :type Integer) (numberOfMove :type Integer))
  (locals (position :type "Vector Structure"))
  (bind _output_get (set `local.position` (`self.K2_GetActorLocation` (`BlueprintMapLibrary.Map_Find` (`self.frameInThisLevel`) IDFrame))))
  (`/Game/Blueprint/BP_Player.MovePlayer` (`local.player`) _output_get (`local.IDFrame`) (`local.numberOfMove`)))

(fn `NoEffect`
  (params (player :type "/Game/Blueprint/BP_Player Object Reference")))

(fn `OnPlayerOnFrame`
  (params (frameType :type "/Game/Datas/Struct_FrameType Structure") (player :type "/Game/Blueprint/BP_Player Object Reference"))
  (`self.DoEvent` frameType player))

(fn `RemoveToPlayerMovement`
  (params (player :type "/Game/Blueprint/BP_Player Object Reference") (numberOfMove :type Integer))
  (locals (actualPosition :type Integer) (positionToMove :type Integer))
  (if (> numberOfMove 0)
    (bind _output_get (set `local.actualPosition` (`/Game/Blueprint/BP_Player.playerPosition` (`local.player`))))
    (bind _backid (`/Game/Blueprint/BP_Frame.ReturnLastID` (`BlueprintMapLibrary.Map_Find` (`self.frameInThisLevel`) _output_get)))
    (set `local.positionToMove` _backid)
    (`self.BackMovePlayers` (`local.player`) (`local.positionToMove`) (`local.numberOfMove`))
    (else
      (bind _output_get_2 (set `local.actualPosition` (`/Game/Blueprint/BP_Player.playerPosition` (`local.player`))))
      (`self.OnPlayerOnFrame` (`/Game/Blueprint/BP_Frame.eventType` (`BlueprintMapLibrary.Map_Find` (`self.frameInThisLevel`) _output_get_2)) (`local.player`)))))

(fn `Shop`
  (params (player :type "/Game/Blueprint/BP_Player Object Reference")))

(fn `Teleport`
  (params (frameID :type Integer) (player :type "/Game/Blueprint/BP_Player Object Reference")))

(fn `UserConstructionScript`)