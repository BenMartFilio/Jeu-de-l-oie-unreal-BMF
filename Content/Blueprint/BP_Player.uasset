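; BP_Player is a board game pawn that holds its order, position and money and slides between board frames.
; On BeginPlay it restores its PlayerID entry from GI_CommonData, or initializes one with an order from Dice; EndOfGame clears it.
; MovePlayer and BackMovePlayer start a Tick-driven lerp timed by the shared move duration.
; Each arrival updates the position and passes the decremented move count to BoardGestion for forward or backward movement.
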(event `self.ReceiveBeginPlay`
  (`self.StartSetup`))

(event `self.ReceiveTick`
  (params (DeltaSeconds :type "Float (single-precision)"))
  (set `self.deltaTime` DeltaSeconds)
  (if (`self.isMoving`)
    (bind _end (`self.MovingFonction`))
    (if _end
      (set `self.isMoving` false)
      (`self.K2_SetActorLocation` (`self.Move To`))
      (set `self.playerPosition` (`self.New Frame ID`))
      (`/Game/Blueprint/BP_BoardGestion.AddToPlayerMovement` (`self.boardGestion`) self (- (`self.Number Of Move`) 1)))
    (elif (`self.isMovingBack`)
      (bind _end_2 (`self.MovingFonction`))
      (if _end_2
        (set `self.isMovingBack` false)
        (`self.K2_SetActorLocation` (`self.Move To`))
        (set `self.playerPosition` (`self.New Frame ID`))
        (`/Game/Blueprint/BP_BoardGestion.RemoveToPlayerMovement` (`self.boardGestion`) self (- (`self.Number Of Move`) 1))))))

(fn `BackMovePlayer`
  (params (MoveTo :type "Vector Structure") (NewFrameID :type Integer) (numberOfMove :type Integer))
  (set `self.Move To` MoveTo)
  (set `self.New Frame ID` NewFrameID)
  (set `self.Number Of Move` numberOfMove)
  (set `self.StartPositio` (`self.K2_GetActorLocation`))
  (set `self.I_0` 0.0)
  (set `self.isMovingBack` true))

(fn `DefineOrder`
  (params (order :type Integer))
  (bind _output_get (set `self.playerOrder` order))
  (`KismetSystemLibrary.PrintString` (`KismetTextLibrary.Conv_TextToString` (`|FormatText` "Je suis {var}" _output_get))))

(fn `EndOfGame`
  (`KismetArrayLibrary.Array_Set` (`/Game/Blueprint/GI_CommonData.PlayerDatas` (`self.commonDatas`)) (`self.playerID`) (make `/Game/Datas/Struct_PlayerData` :`isInitialized` false)))

(fn `MovePlayer`
  (params (MoveTo :type "Vector Structure") (NewFrameID :type Integer) (numberOfMove :type Integer))
  (locals (tempsDeplacement :type "Float (double-precision)") (StartPosition :type "Vector Structure") (i :type "Float (double-precision)"))
  (set `self.Move To` MoveTo)
  (set `self.New Frame ID` NewFrameID)
  (set `self.Number Of Move` numberOfMove)
  (set `self.StartPositio` (`self.K2_GetActorLocation`))
  (set `self.I_0` 0.0)
  (set `self.isMoving` true))

(fn `MovingFonction`
  (returns (End :type Boolean))
  (locals (tempsDeplacement :type "Float (double-precision)" :default 0.0))
  (set `local.tempsDeplacement` (`/Game/Blueprint/GI_CommonData.DeplacementDuree` (`self.commonDatas`)))
  (if (< (`self.I_0`) 1.0)
    (`self.K2_SetActorLocation` (`KismetMathLibrary.VLerp` (`self.StartPositio`) (`self.Move To`) (`self.I_0`)))
    (set `self.I_0` (+ (`self.I_0`) (/ (`self.deltaTime`) (`local.tempsDeplacement`))))
    (return false)
    (else
      (return true))))

(fn `StartSetup`
  (locals (playerData :type "/Game/Datas/Struct_PlayerData Structure"))
  (bind (_order _position _isitmyturn _money) (break `/Game/Datas/Struct_PlayerData` (`local.playerData`)))
  (bind _asgi_common_data (cast `/Game/Blueprint/GI_CommonData` (`GameplayStatics.GetGameInstance`))
    (:`then`
      (set `self.commonDatas` _asgi_common_data)
      (if (or (< (`self.playerID`) 0) (>= (`self.playerID`) (`KismetArrayLibrary.Array_Length` (`/Game/Blueprint/GI_CommonData.PlayerDatas` (`self.commonDatas`)))))
        (`KismetSystemLibrary.PrintString` "PlayerID invalide")
        (else
          (bind _output_get (set `local.playerData` (`|GetArrayItem` (`/Game/Blueprint/GI_CommonData.PlayerDatas` (`self.commonDatas`)) (`self.playerID`))))
          (if (`.isInitialized_17_47A13B1B49C0F549B8F51C80A1D7A7D5` (break `/Game/Datas/Struct_PlayerData` _output_get))
            (set `self.playerPosition` _position)
            (set `self.playerOrder` _order)
            (set `self.playerMoney` _money)
            (else
              (bind _orderout (`/Game/Blueprint/BP_Dice.GetPlayers` (`self.dice`) self))
              (set `self.playerOrder` _orderout)
              (`KismetArrayLibrary.Array_Set` (`/Game/Blueprint/GI_CommonData.PlayerDatas` (`self.commonDatas`)) (`self.playerID`) (make `/Game/Datas/Struct_PlayerData` :`Order` (`self.playerOrder`) :`Position` (`self.playerPosition`) :`Money` (`self.playerMoney`) :`isInitialized` true)))))))
    (:`CastFailed`
      (`KismetSystemLibrary.PrintString` "CommonData invalide"))))

(fn `UserConstructionScript`)