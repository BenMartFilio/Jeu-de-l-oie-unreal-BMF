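; BP_Camera is the Blueprint that handles player input and HUD setup for a dice-based, turn-ordered game.
; On BeginPlay it adds the IMC_General mapping context, caches the level's BP_Dice actor and adds WBP_HUD to the viewport.
; The IA_Space input prints a debug string and calls ThrowDice for a six-sided roll, passing the dice's own next-player order as the player ID.
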(event `self.ReceiveBeginPlay`
  (`EnhancedInputSubsystemInterface.AddMappingContext` (pcsubsystem `EnhancedInputLocalPlayerSubsystem` (`GameplayStatics.GetPlayerController` 0)) "/Game/Inputs/IMC_General.IMC_General" 0 (struct))
  (bind _returnvalue (`GameplayStatics.GetActorOfClass` "/Game/Blueprint/BP_Dice.BP_Dice_C"))
  (set `self.dice` _returnvalue)
  (bind _returnvalue_2 (`|CreateWidget` "/Game/Widget/WBP_HUD.WBP_HUD_C"))
  (`UserWidget.AddToViewport` _returnvalue_2 0))

(event `EnhancedInput|/Game/Inputs/IA_Space`
  (params (ActionValue :type Boolean) (ElapsedSeconds :type "Float (double-precision)") (TriggeredSeconds :type "Float (double-precision)") (InputAction :type "InputAction Object Reference" :default "/Game/Inputs/IA_Space.IA_Space"))
  (bind _dice (`self.dice`))
  (:`Started`
    (`KismetSystemLibrary.PrintString` "ESPACE")
    (`/Game/Blueprint/BP_Dice.ThrowDice` _dice (`/Game/Blueprint/BP_Dice.NextPlayerOrdrer` _dice) 6)))

(fn `UserConstructionScript`)