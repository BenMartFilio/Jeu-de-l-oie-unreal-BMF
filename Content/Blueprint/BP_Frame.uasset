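; BP_Frame is a path frame actor that knows its own order ID, its previous frame and one or more next frames.
; On BeginPlay it pushes its ColorID to the mesh materials as the ColorIDIndex scalar parameter.
; Getter functions expose the IDs, with ReturnNextID printing an error and returning zero if none is set.
; Branching goes through ChoicePath, a placeholder that currently always takes the first next ID.
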(event `self.ReceiveBeginPlay`
  (`self.DefineColor`))

(fn `ChoicePath`
  (returns (NextFrame :type Integer))
  ; Faire le système de choix ici
  (return (`|GetArrayItem` (`self.NextID`))))

(fn `DefineColor`
  (`MeshComponent.SetScalarParameterValueOnMaterials` (`self.Mesh`) "ColorIDIndex" (`KismetMathLibrary.Conv_IntToDouble` (`self.ColorID`))))

(fn `ReturnFrameID`
  (returns (FrameID :type Integer))
  (return (`self.OrderID`)))

(fn `ReturnLastID`
  (returns (BackID :type Integer))
  (return (`self.BackID`)))

(fn `ReturnNextID`
  (returns (NextID :type Integer))
  (if (== (`KismetArrayLibrary.Array_Length` (`self.NextID`)) 1)
    (return (`|GetArrayItem` (`self.NextID`)))
    (elif (> (`KismetArrayLibrary.Array_Length` (`self.NextID`)) 1)
      (bind _nextframe (`self.ChoicePath`))
      (return _nextframe)
      (else
        (`KismetSystemLibrary.PrintString` "\"ERREUR, nextID de la frame ID : \" + OrderID + \" n'est pas défini.\"")
        (return 0)))))

(fn `UserConstructionScript`)