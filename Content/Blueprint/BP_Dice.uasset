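; Dice actor for a board game that rolls movement and tracks which player acts next.
; On BeginPlay it restores the turn from the flagged player's array index in GI_CommonData, rewriting that entry without the turn flag.
; GetPlayers assigns each player an incrementing order and maps it.
; ThrowDice prints a random roll, sends that player's move to BoardGestion, then advances the wrapping turn counter.
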(event `self.ReceiveBeginPlay`
  (bind _asgi_common_data (cast `/Game/Blueprint/GI_CommonData` (`GameplayStatics.GetGameInstance`)))
  (set `self.commonDatas` _asgi_common_data)
  (`self.OnLoadLevel`))

(fn `GetPlayers`
  (params (player :type "/Game/Blueprint/BP_Player Object Reference"))
  (returns (OrderOut :type Integer))
  (locals (order :type Integer))
  (bind _result (`/Engine/EditorBlueprintResources/StandardMacros.IncrementInt` (`self.OrderIncrement`))
    (:`  `
      (bind _output_get (set `local.order` _result))
      (`/Game/Blueprint/BP_Player.DefineOrder` player _output_get)
      (`BlueprintMapLibrary.Map_Add` (`self.playersAndOrder`) _output_get player)
      (return (`local.order`)))))

(fn `MoveOnBoard`
  (params (numberOfMove :type Integer) (playerOrderID :type Integer))
  (`/Game/Blueprint/BP_BoardGestion.AddToPlayerMovement` (`self.boardGestion`) (`BlueprintMapLibrary.Map_Find` (`self.playersAndOrder`) playerOrderID) numberOfMove))

(fn `OnLoadLevel`
  (for (_array_element _array_index) (`/Game/Blueprint/GI_CommonData.PlayerDatas` (`self.commonDatas`))
    (bind (_order _position _isitmyturn _money _inventory _isinitialized) (break `/Game/Datas/Struct_PlayerData` _array_element))
    (if _isitmyturn
      (set `self.NextPlayerOrdrer` _array_index)
      (`KismetArrayLibrary.Array_Set` (`/Game/Blueprint/GI_CommonData.PlayerDatas` (`self.commonDatas`)) _array_index (make `/Game/Datas/Struct_PlayerData` _order _position false _money _inventory _isinitialized)))))

(fn `ThrowDice`
  (params (PlayerOrderID :type Integer) (NumberFaceOfDice :type Integer :default 6))
  (locals (DiceResult :type Integer))
  (bind _output_get (set `local.DiceResult` (`KismetMathLibrary.RandomIntegerInRange` 1 NumberFaceOfDice)))
  (`KismetSystemLibrary.PrintString` (`KismetTextLibrary.Conv_TextToString` (`|FormatText` "Le dé renvoie : {nb}" _output_get)))
  (`self.MoveOnBoard` (`local.DiceResult`) (`local.PlayerOrderID`))
  (set `self.NextPlayerOrdrer` (`KismetMathLibrary.Max` (mod (+ (`self.NextPlayerOrdrer`) 1) (+ (`BlueprintMapLibrary.Map_Length` (`self.playersAndOrder`)) 1)) 1)))

(fn `UserConstructionScript`)